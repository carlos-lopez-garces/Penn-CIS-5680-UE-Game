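; Ruby necklace prop that levitates in place and tracks whether the top-down player character is in range.
; On BeginPlay, a Levitation timeline moves it vertically around its starting position using a scaled sine of its ZOffset track.
; Sphere collider and mesh overlaps share one IsPlayerInRange flag, so leaving either clears it.
; The flag is only set here, never read.
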(event `self.ReceiveBeginPlay`
  (set `self.InitialPosition` (`self.K2_GetActorLocation`))
  (bind (_direction _zoffset) (`Timeline|Levitation`)
    (:`Update`
      (`self.K2_SetActorLocation` (`KismetMathLibrary.MakeVector` (.x (`self.InitialPosition`)) (.y (`self.InitialPosition`)) (+ (* (`KismetMathLibrary.Sin` _zoffset) 100.0) (.z (`self.InitialPosition`))))))))

(event `self.SphereCollider.OnComponentBeginOverlap`
  (params (OverlappedComponent :type "PrimitiveComponent Object Reference") (OtherActor :type "Actor Object Reference") (OtherComp :type "PrimitiveComponent Object Reference") (OtherBodyIndex :type Integer) (bFromSweep :type Boolean) (SweepResult :type "HitResult Structure (by ref)"))
  (cast `/Game/TopDown/Blueprints/BP_TopDownCharacter` OtherActor)
  (set `self.IsPlayerInRange` true :!label _label))

(event `self.SphereCollider.OnComponentEndOverlap`
  (params (OverlappedComponent :type "PrimitiveComponent Object Reference") (OtherActor :type "Actor Object Reference") (OtherComp :type "PrimitiveComponent Object Reference") (OtherBodyIndex :type Integer))
  (cast `/Game/TopDown/Blueprints/BP_TopDownCharacter` OtherActor)
  (set `self.IsPlayerInRange` false :!label _label_2))

(event `self.StaticMesh.OnComponentBeginOverlap`
  (params (OverlappedComponent :type "PrimitiveComponent Object Reference") (OtherActor :type "Actor Object Reference") (OtherComp :type "PrimitiveComponent Object Reference") (OtherBodyIndex :type Integer) (bFromSweep :type Boolean) (SweepResult :type "HitResult Structure (by ref)"))
  (cast `/Game/TopDown/Blueprints/BP_TopDownCharacter` OtherActor)
  (goto _label))

(event `self.StaticMesh.OnComponentEndOverlap`
  (params (OverlappedComponent :type "PrimitiveComponent Object Reference") (OtherActor :type "Actor Object Reference") (OtherComp :type "PrimitiveComponent Object Reference") (OtherBodyIndex :type Integer))
  (cast `/Game/TopDown/Blueprints/BP_TopDownCharacter` OtherActor)
  (goto _label_2))

(fn `UserConstructionScript`)
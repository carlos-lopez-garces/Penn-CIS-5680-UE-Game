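; Guard AI character that patrols points and watches for the top-down player character, reporting sightings to its guard controller.
; Each tick it sphere-traces along LookDir for pawns, keeps those within a 45-degree half-angle, then line-traces for occlusion before calling CanSeePlayer with the player or empty.
; Helpers set walk speed and return the next patrol point in a looping list; death destroys the actor.
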(event `Death`
  (`self.K2_DestroyActor`))

(event `self.ReceivePossessed`
  (params (NewController :type "Controller Object Reference"))
  (set `self.As BP Guard Controller` (cast `/Game/AI/BP_Guard_Controller` NewController :!pure true)))

(event `self.ReceiveTick`
  (params (DeltaSeconds :type "Float (single-precision)"))
  (bind _lookdir (`self.LookDir`))
  (bind _as_bp_guard_controller (`self.As BP Guard Controller`))
  (bind _returnvalue (`SceneComponent.K2_GetComponentLocation` _lookdir))
  (if (!= (`self.As BP Guard Controller`) null)
    (bind (_outhits _returnvalue_2) (`KismetSystemLibrary.SphereTraceMultiForObjects` :`Start` _returnvalue :`End` (+ _returnvalue (* (`SceneComponent.GetForwardVector` _lookdir) (`self.SightRange`))) :`Radius` 500.0 :`ObjectTypes` (`self.PawnType`) :`DrawTime` 0.5))
    (for _array_element _outhits
      (bind _asbp_top_down_character (cast `/Game/TopDown/Blueprints/BP_TopDownCharacter` (`.HitActor` (`GameplayStatics.BreakHitResult` _array_element)))
        (:`then`
          (bind _returnvalue_3 (`self.K2_GetActorLocation` _asbp_top_down_character))
          (if (<= (`KismetMathLibrary.DegAcos` (`KismetMathLibrary.Dot_VectorVector` (`SceneComponent.GetForwardVector` (`self.LookDir`)) (`KismetMathLibrary.Normal` (- _returnvalue_3 (`self.K2_GetActorLocation`))))) 45.0)
            (bind _outhit (`KismetSystemLibrary.LineTraceSingleForObjects` :`Start` (`SceneComponent.K2_GetComponentLocation` (`self.LookDir`)) :`End` _returnvalue_3 :`ObjectTypes` (`self.OtherBlockingObjects`) :`DrawDebugType` "ForDuration" :`DrawTime` 0.5))
            (bind _asbp_top_down_character_2 (cast `/Game/TopDown/Blueprints/BP_TopDownCharacter` (`.HitActor` (`GameplayStatics.BreakHitResult` _outhit)))
              (:`then`
                (`/Game/AI/BP_Guard_Controller.CanSeePlayer` _as_bp_guard_controller _asbp_top_down_character_2)
                (break))
              (:`CastFailed`
                (`/Game/AI/BP_Guard_Controller.CanSeePlayer` _as_bp_guard_controller null)))
            (else
              (`/Game/AI/BP_Guard_Controller.CanSeePlayer` (`self.As BP Guard Controller`) null))))
        (:`CastFailed`
          (`/Game/AI/BP_Guard_Controller.CanSeePlayer` (`self.As BP Guard Controller`) null))))
    (if (not _returnvalue_2)
      (`/Game/AI/BP_Guard_Controller.CanSeePlayer` (`self.As BP Guard Controller`) null))))

(fn `GetPatrolPoint`
  (returns (PatrolPos :type "TargetPoint Object Reference"))
  (if true
    (bind _output_get (set `self.PatrolIndex` (mod (+ (`self.PatrolIndex`) 1) (`KismetArrayLibrary.Array_Length` (`self.Patrol Points`))))))
  (return (`|GetArrayItem` (`self.Patrol Points`) _output_get)))

(fn `UpdateWalkSpeed`
  (params (NewSpeed :type "Float (double-precision)"))
  (set `CharacterMovementComponent.MaxWalkSpeed` NewSpeed (`self.CharacterMovement`)))

(fn `UserConstructionScript`)
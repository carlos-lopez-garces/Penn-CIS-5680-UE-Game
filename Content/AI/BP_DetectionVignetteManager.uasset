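; Actor that fades a screen vignette in and out to show whether the player is detected.
; Construction creates a dynamic instance of M_Vignette and sets it as a blendable on its PostProcess component.
; Each tick, a clamped transition value rises or falls with IsPlayerDetected over a configurable time and lerps between minimum and maximum intensity.
; UpdateVignette writes the result to the material's VignetteIntensity parameter.
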(event `self.ReceiveTick`
  (params (DeltaSeconds :type "Float (single-precision)"))
  (if (`self.IsPlayerDetected`)
    (bind _output_get (set `self.CurrVignetteTransition` (`KismetMathLibrary.FClamp` (+ (`self.CurrVignetteTransition`) (/ DeltaSeconds (`self.VignetteTransitionSpeed`))))))
    (`self.UpdateVignette` (`KismetMathLibrary.Lerp` (`self.MinVignetteIntensity`) (`self.MaxVignetteIntensity`) _output_get))
    (else
      (bind _output_get_2 (set `self.CurrVignetteTransition` (`KismetMathLibrary.FClamp` (- (`self.CurrVignetteTransition`) (/ DeltaSeconds (`self.VignetteTransitionSpeed`))))))
      (`self.UpdateVignette` (`KismetMathLibrary.Lerp` (`self.MinVignetteIntensity`) (`self.MaxVignetteIntensity`) _output_get_2)))))

(fn `UpdateVignette`
  (params (NewIntensity :type "Float (double-precision)"))
  (bind _asmaterial_instance_dynamic (cast `MaterialInstanceDynamic` (`.Object` (break `WeightedBlendable` (`|GetArrayItem` (`.Array` (break `WeightedBlendables` (`.WeightedBlendables` (break `PostProcessSettings` (`PostProcessComponent.Settings` (`self.PostProcess`)))))))))))
  (`MaterialInstanceDynamic.SetScalarParameterValue` _asmaterial_instance_dynamic "VignetteIntensity" NewIntensity))

(fn `UserConstructionScript`
  (bind _returnvalue (`KismetMaterialLibrary.CreateDynamicMaterialInstance` "/Game/AI/M_Vignette.M_Vignette"))
  (bind _output_get (set `self.VignetteMaterial` _returnvalue))
  (setmembers `PostProcessSettings` :`StructRef` (`PostProcessComponent.Settings` (`self.PostProcess`)) :`WeightedBlendables` (make `WeightedBlendables` (`|MakeArray` (make `WeightedBlendable` 1.0 _output_get)))))
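; AI controller for guards that detects the player, respecting shadows, and feeds the result to the BT_Guard behavior tree.
; CanSeePlayer stores the seen actor, and Tick sets the line-of-sight and target Blackboard keys and calls DetectPlayer while that actor is out of shadow.
; With no actor seen, a timer delays losing sight, then clears those keys and calls StopDetecting on the player found at BeginPlay.
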(event `self.ReceivePossess`
  (params (PossessedPawn :type "Pawn Object Reference"))
  (`self.RunBehaviorTree` "/Game/AI/BT_Guard.BT_Guard"))

(event `self.ReceiveBeginPlay`
  (bind _returnvalue (`GameplayStatics.GetActorOfClass` "/Game/TopDown/Blueprints/BP_TopDownCharacter.BP_TopDownCharacter_C"))
  (set `self.PlayerActorDoNotUse` _returnvalue))

(event `CanSeePlayer`
  (params (Actor :type "/Game/TopDown/Blueprints/BP_TopDownCharacter Object Reference"))
  (bind _output_get (set `self.ActorSeen` Actor))
  (set `self.WasActorSeen?` (!= _output_get null)))

(event `self.ReceiveTick`
  (params (DeltaSeconds :type "Float (single-precision)"))
  (bind _returnvalue (`AIBlueprintHelperLibrary.GetBlackboard` null))
  (bind _actorseen (`self.ActorSeen`))
  (if (`self.WasActorSeen?`)
    (if (not (`/Game/TopDown/Blueprints/BP_TopDownCharacter.IsInShadow` (`self.ActorSeen`)))
      (`KismetSystemLibrary.K2_ClearAndInvalidateTimerHandle` (`self.Enemy Timer`))
      (`BlackboardComponent.SetValueAsBool` _returnvalue (`self.HasLineOfSight`) true)
      (`BlackboardComponent.SetValueAsObject` _returnvalue (`self.PlayerActor`) _actorseen)
      (`/Game/TopDown/Blueprints/BP_TopDownCharacter.DetectPlayer` _actorseen self))
    (elif (not (`KismetSystemLibrary.K2_IsValidTimerHandle` (`self.Enemy Timer`)))
      (bind _returnvalue_2 (`KismetSystemLibrary.K2_SetTimerDelegate` (delegate `Enemy Lost Sight`) (`self.Line of Sight Timer`)))
      (set `self.Enemy Timer` _returnvalue_2))))

(event `Enemy Lost Sight`
  (bind _returnvalue (`AIBlueprintHelperLibrary.GetBlackboard` null))
  (`BlackboardComponent.SetValueAsBool` _returnvalue (`self.HasLineOfSight`) false)
  (`BlackboardComponent.SetValueAsObject` _returnvalue (`self.PlayerActor`) null)
  (`/Game/TopDown/Blueprints/BP_TopDownCharacter.StopDetecting` (`self.PlayerActorDoNotUse`) self))

(fn `UserConstructionScript`)
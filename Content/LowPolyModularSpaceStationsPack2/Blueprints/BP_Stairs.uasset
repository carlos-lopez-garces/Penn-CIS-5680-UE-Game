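; BP_Stairs is a modular staircase actor for space station levels, built procedurally in its construction script with no active event logic.
; It adds copies of the base step mesh up to StepsCount, placing each relative to the previous one with a configurable horizontal offset and fixed rise.
; It then sets the custom-color material flag on all steps, base included, and runs CustomColorFunction on each.
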(fn `UserConstructionScript`
  (bind _newstepcomponents (`self.NewStepComponents`))
  (`parent.UserConstructionScript`)
  (`|ExecutionSequence`
    (:`then_0`
      (`KismetArrayLibrary.Array_Clear` (`self.NewStepComponents`))
      (for _index (range (+ (- (`self.StepsCount`) 2) 1))
        (bind _returnvalue_location (`KismetMathLibrary.BreakTransform` (`SceneComponent.GetRelativeTransform` (`|GetArrayItem` (`self.NewStepComponents`) (- _index 1)))))
        (bind _returnvalue (`AddComponent|NODE_AddStaticMeshComponent-0` :`RelativeTransform` (`KismetMathLibrary.Conv_VectorToTransform` (`KismetMathLibrary.MakeVector` (- (.x _returnvalue_location) (`self.NextStepHorizontalOffset`)) (.y _returnvalue_location) (+ (.z _returnvalue_location) 20.0)))))
        (`StaticMeshComponent.SetStaticMesh` _returnvalue (`StaticMeshComponent.StaticMesh` (`self.SM_BaseMesh`)))
        (`KismetArrayLibrary.Array_Add` (`self.NewStepComponents`) _returnvalue)))
    (:`then_1`
      (`KismetArrayLibrary.Array_Add` _newstepcomponents (`self.SM_BaseMesh`))
      (`MeshComponent.SetScalarParameterValueOnMaterials` _newstepcomponents "isCustomColors" (`KismetMathLibrary.Conv_BoolToDouble` (`self.isCustomColors`)))
      (for _array_element _newstepcomponents
        (`self.CustomColorFunction` _array_element)))))
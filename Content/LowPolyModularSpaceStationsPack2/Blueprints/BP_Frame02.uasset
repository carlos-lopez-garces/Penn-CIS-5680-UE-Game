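; BP_Frame02 is a modular space station frame with a sliding door that responds to overlaps on its OpenCollision volume.
; Begin and end overlap play and reverse the DoorOpening timeline, whose track feeds DoorPosition to slide the door along local Y, clamped to MaxOpenDistance.
; The Construction Script applies emissive and glass settings to the frame, plus optional custom colors to frame and door through per-slot dynamic material instances.
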(event `self.OpenCollision.OnComponentBeginOverlap`
  (params (OverlappedComponent :type "PrimitiveComponent Object Reference") (OtherActor :type "Actor Object Reference") (OtherComp :type "PrimitiveComponent Object Reference") (OtherBodyIndex :type Integer) (bFromSweep :type Boolean) (SweepResult :type "HitResult Structure (by ref)"))
  (if (`self.isDoorClosed`)
    (`TimelineComponent.Play` (`self.DoorOpening`))
    (set `self.isDoorClosed` false)))

(event `self.OpenCollision.OnComponentEndOverlap`
  (params (OverlappedComponent :type "PrimitiveComponent Object Reference") (OtherActor :type "Actor Object Reference") (OtherComp :type "PrimitiveComponent Object Reference") (OtherBodyIndex :type Integer))
  (if (not (`self.isDoorClosed`))
    (`TimelineComponent.Reverse` (`self.DoorOpening`))
    (set `self.isDoorClosed` true)))

(fn `CustomColorFunction`
  (params (Target :type "PrimitiveComponent Object Reference"))
  (bind _returnvalue (`PrimitiveComponent.CreateDynamicMaterialInstance` Target 0 (`PrimitiveComponent.GetMaterial` Target 0) "None"))
  (`MaterialInstanceDynamic.SetVectorParameterValue` _returnvalue "CustomColor" (`self.ColorMatID_00`))
  (bind _returnvalue_2 (`PrimitiveComponent.CreateDynamicMaterialInstance` Target 1 (`PrimitiveComponent.GetMaterial` Target 1) "None"))
  (`MaterialInstanceDynamic.SetVectorParameterValue` _returnvalue_2 "CustomColor" (`self.ColorMatID_01`))
  (bind _returnvalue_3 (`PrimitiveComponent.CreateDynamicMaterialInstance` Target 2 (`PrimitiveComponent.GetMaterial` Target 2) "None"))
  (`MaterialInstanceDynamic.SetVectorParameterValue` _returnvalue_3 "CustomColor" (`self.ColorMatID_02`))
  (bind _returnvalue_4 (`PrimitiveComponent.CreateDynamicMaterialInstance` Target 3 (`PrimitiveComponent.GetMaterial` Target 3) "None"))
  (`MaterialInstanceDynamic.SetVectorParameterValue` _returnvalue_4 "CustomColor" (`self.ColorMatID_03`))
  (bind _returnvalue_5 (`PrimitiveComponent.CreateDynamicMaterialInstance` Target 4 (`PrimitiveComponent.GetMaterial` Target 4) "None"))
  (`MaterialInstanceDynamic.SetVectorParameterValue` _returnvalue_5 "CustomColor" (`self.ColorMatID_04`)))

(fn `DoorPosition`
  (bind _maxopendistance (`self.MaxOpenDistance`))
  (`SceneComponent.K2_SetRelativeLocation` (`self.SM_Door01`) (`KismetMathLibrary.MakeVector` 0.0 (* -1 (`KismetMathLibrary.FClamp` (* (`self.OpenPercent`) (/ _maxopendistance 100.0)) 0.0 _maxopendistance))) false false))

(fn `UserConstructionScript`
  (bind _sm_basemesh (`self.SM_BaseMesh`))
  (bind _sm_basemesh_2 (`self.SM_BaseMesh`))
  (`|ExecutionSequence`
    (:`then_0`
      (`MeshComponent.SetScalarParameterValueOnMaterials` _sm_basemesh "EmissivePower" (`self.EmissivePower`))
      (`MeshComponent.SetVectorParameterValueOnMaterials` _sm_basemesh "EmissiveColor" (`KismetMathLibrary.Conv_LinearColorToVector` (`self.EmissiveColor`))))
    (:`then_3`
      (`MeshComponent.SetScalarParameterValueOnMaterials` (`self.SM_BaseMesh`) "isCustomColors" (`KismetMathLibrary.Conv_BoolToDouble` (`self.isCustomColors`)))
      (`MeshComponent.SetScalarParameterValueOnMaterials` (`self.SM_Door01`) "isCustomColors" (`KismetMathLibrary.Conv_BoolToDouble` (`self.isCustomColors`)))
      (`self.CustomColorFunction` (`self.SM_Door01`))
      (`self.CustomColorFunction` (`self.SM_BaseMesh`)))
    (:`then_4`
      (`MeshComponent.SetScalarParameterValueOnMaterials` _sm_basemesh_2 "GlassOpacity" (`self.GlassOpacity`))
      (`MeshComponent.SetVectorParameterValueOnMaterials` _sm_basemesh_2 "GlassColor" (`KismetMathLibrary.Conv_LinearColorToVector` (`self.GlassColor`))))))
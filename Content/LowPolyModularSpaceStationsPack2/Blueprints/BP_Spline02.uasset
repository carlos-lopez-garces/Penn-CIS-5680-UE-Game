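; Spline-driven modular mesh actor from a low-poly space station pack that lays a configurable static mesh along an editable spline.
; The construction script adds one spline mesh per segment, matching point locations and tangents, and collects them in an array.
; It then gives six material slots dynamic instances with per-slot custom colors and sets custom-color toggle and emissive color and power parameters.
; The event graph has no runtime logic.
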(fn `CustomColorFunction`
  (params (Target :type "PrimitiveComponent Object Reference"))
  (bind _returnvalue (`PrimitiveComponent.CreateDynamicMaterialInstance` Target 0 (`PrimitiveComponent.GetMaterial` Target 0) "None"))
  (`MaterialInstanceDynamic.SetVectorParameterValue` _returnvalue "CustomColor" (`self.ColorMatID_00`))
  (bind _returnvalue_2 (`PrimitiveComponent.CreateDynamicMaterialInstance` Target 1 (`PrimitiveComponent.GetMaterial` Target 1) "None"))
  (`MaterialInstanceDynamic.SetVectorParameterValue` _returnvalue_2 "CustomColor" (`self.ColorMatID_01`))
  (bind _returnvalue_3 (`PrimitiveComponent.CreateDynamicMaterialInstance` Target 2 (`PrimitiveComponent.GetMaterial` Target 2) "None"))
  (`MaterialInstanceDynamic.SetVectorParameterValue` _returnvalue_3 "CustomColor" (`self.ColorMatID_02`))
  (bind _returnvalue_4 (`PrimitiveComponent.CreateDynamicMaterialInstance` Target 3 (`PrimitiveComponent.GetMaterial` Target 3) "None"))
  (`MaterialInstanceDynamic.SetVectorParameterValue` _returnvalue_4 "CustomColor" (`self.ColorMatID_03`))
  (bind _returnvalue_5 (`PrimitiveComponent.CreateDynamicMaterialInstance` Target 4 (`PrimitiveComponent.GetMaterial` Target 4) "None"))
  (`MaterialInstanceDynamic.SetVectorParameterValue` _returnvalue_5 "CustomColor" (`self.ColorMatID_04`))
  (bind _returnvalue_6 (`PrimitiveComponent.CreateDynamicMaterialInstance` Target 5 (`PrimitiveComponent.GetMaterial` Target 5) "None"))
  (`MaterialInstanceDynamic.SetVectorParameterValue` _returnvalue_6 "CustomColor" (`self.ColorMatID_05`)))

(fn `UserConstructionScript`
  (bind _spline (`self.Spline`))
  (bind _splinesbodies (`self.SplinesBodies`))
  (`|ExecutionSequence`
    (:`then_0`
      (for _index (range (+ (- (`SplineComponent.GetNumberOfSplinePoints` _spline) 2) 1))
        (bind _returnvalue (`AddComponent|NODE_AddSplineMeshComponent-0`))
        (`StaticMeshComponent.SetStaticMesh` _returnvalue (`self.SM_SplineMesh_Body`))
        (`SplineMeshComponent.SetForwardAxis` _returnvalue (`self.forward_axis`) true)
        (`SceneComponent.K2_AttachToComponent` _returnvalue (`self.Spline`) "None" "SnapToTarget" "SnapToTarget" "SnapToTarget" true)
        (bind _returnvalue_2 (+ _index 1))
        (`SplineMeshComponent.SetStartAndEnd` _returnvalue (`SplineComponent.GetLocationAtSplinePoint` _spline _index "Local") (`SplineComponent.GetTangentAtSplinePoint` _spline _index "Local") (`SplineComponent.GetLocationAtSplinePoint` _spline _returnvalue_2 "Local") (`SplineComponent.GetTangentAtSplinePoint` _spline _returnvalue_2 "Local") true)
        (`KismetArrayLibrary.Array_Add` (`self.SplinesBodies`) _returnvalue)))
    (:`then_1`
      (for _array_element _splinesbodies
        (`self.CustomColorFunction` _array_element)))
    (:`then_2`
      (`MeshComponent.SetScalarParameterValueOnMaterials` _splinesbodies "isCustomColors" (`KismetMathLibrary.Conv_BoolToDouble` (`self.isCustomColors`))))
    (:`then_3`
      (`MeshComponent.SetScalarParameterValueOnMaterials` _splinesbodies "EmissivePower" (`self.EmissivePower`))
      (`MeshComponent.SetVectorParameterValueOnMaterials` _splinesbodies "EmissiveColor" (`KismetMathLibrary.Conv_LinearColorToVector` (`self.EmissiveColor`))))))